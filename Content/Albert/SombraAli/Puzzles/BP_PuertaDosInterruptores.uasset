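; Puzzle door actor that opens while either of its two switches is held down.
; Four custom events set and clear a pressed flag for each switch, with no callers in this graph.
; Every Tick polls both flags with an OR, hiding the Puerta component and disabling its collision when open, otherwise showing it with query-only collision.
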(event `self.ReceiveTick`
  (params (DeltaSeconds :type "Float (single-precision)"))
  (if (or (`self.Interruptor2Pulsado`) (`self.Interruptor1Pulsado`))
    (`SceneComponent.SetVisibility` (`self.Puerta`) false false)
    (`PrimitiveComponent.SetCollisionEnabled` (`self.Puerta`) "NoCollision")
    (else
      (`SceneComponent.SetVisibility` (`self.Puerta`) true false)
      (`PrimitiveComponent.SetCollisionEnabled` (`self.Puerta`) "QueryOnly"))))

(event `PulsarInterruptor1`
  (set `self.Interruptor1Pulsado` true))

(event `PulsarInterruptor2`
  (set `self.Interruptor2Pulsado` true))

(event `DejarDePulsarInterruptor1`
  (set `self.Interruptor1Pulsado` false))

(event `DejarDePulsarInterruptor2`
  (set `self.Interruptor2Pulsado` false))

(fn `UserConstructionScript`)