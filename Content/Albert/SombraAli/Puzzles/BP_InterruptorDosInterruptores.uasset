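; Pressure switch for a two-switch door puzzle, held down by either the Ali character or the Sombra Ali shadow.
; Every Tick it polls its Box for both classes, prints debug text and fires a pressed or released event, repeating each frame rather than on change.
; Those events look up the first BP_PuertaDosInterruptores tagged NombrePuerta and call its press or release function for switch 1 or 2, chosen by NumeroInterruptor.
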(event `self.ReceiveTick`
  (params (DeltaSeconds :type "Float (single-precision)"))
  (bind _returnvalue (> (`KismetArrayLibrary.Array_Length` (`PrimitiveComponent.GetOverlappingActors` (`self.Box`) "/Game/Albert/SombraAli/BP_SombraAli.BP_SombraAli_C")) 0))
  (bind _returnvalue_2 (> (`KismetArrayLibrary.Array_Length` (`PrimitiveComponent.GetOverlappingActors` (`self.Box`) "/Game/Albert/SombraAli/BP_ThirdPersonCharacterAli.BP_ThirdPersonCharacterAli_C")) 0))
  (`|ExecutionSequence`
    (:`then_0`
      (if _returnvalue_2
        (`KismetSystemLibrary.PrintString` "Overlap Third Person" true true (struct :`G` 1.0 :`B` 0.052975 :`A` 1.0))
        (`self.InterruptorPulsado`)))
    (:`then_1`
      (if _returnvalue
        (`KismetSystemLibrary.PrintString` "Overlap Sombra" true true (struct :`R` 0.144441 :`B` 1.0 :`A` 1.0))
        (`self.InterruptorPulsado`)))
    (:`then_2`
      (if (and (not _returnvalue_2) (not _returnvalue))
        (`KismetSystemLibrary.PrintString` "Cerrar puerta" true true (struct :`R` 1.0 :`B` 0.06219 :`A` 1.0))
        (`self.InterruptorDejadoDePulsar`)))))

(event `InterruptorPulsado`
  (bind _outactors (`GameplayStatics.GetAllActorsOfClassWithTag` "/Game/Albert/SombraAli/Puzzles/BP_PuertaDosInterruptores.BP_PuertaDosInterruptores_C" (`self.NombrePuerta`)))
  (switch `int` (`self.NumeroInterruptor`)
    (:`1`
      (bind _output (`|GetArrayItem` _outactors))
      (`/Game/Albert/SombraAli/Puzzles/BP_PuertaDosInterruptores.PulsarInterruptor1` _output))
    (:`2`
      (`/Game/Albert/SombraAli/Puzzles/BP_PuertaDosInterruptores.PulsarInterruptor2` _output))))

(event `InterruptorDejadoDePulsar`
  (bind _outactors (`GameplayStatics.GetAllActorsOfClassWithTag` "/Game/Albert/SombraAli/Puzzles/BP_PuertaDosInterruptores.BP_PuertaDosInterruptores_C" (`self.NombrePuerta`)))
  (switch `int` (`self.NumeroInterruptor`)
    (:`1`
      (bind _output (`|GetArrayItem` _outactors))
      (`/Game/Albert/SombraAli/Puzzles/BP_PuertaDosInterruptores.DejarDePulsarInterruptor1` _output))
    (:`2`
      (`/Game/Albert/SombraAli/Puzzles/BP_PuertaDosInterruptores.DejarDePulsarInterruptor2` _output))))

(fn `UserConstructionScript`)