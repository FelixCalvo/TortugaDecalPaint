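; Component that gives its owner a delayed shadow follower and lets the player swap places with it on C.
; A fixed-length buffer, sized by TiempoRetraso and prefilled at BeginPlay, holds owner transforms as a sliding window sampled on a 0.1-second looping timer.
; The spawned BP_SombraAliEquipoArte chases the oldest sample through movement input each Tick.
; A Niagara trail is also attached behind the owner.
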(event `self.ReceiveBeginPlay`
  (`self.InitializePositionData`)
  (`KismetSystemLibrary.K2_SetTimerDelegate` (`|CreateDelegate` :!event `UpdatePositionData`) 0.1 true)
  (bind _returnvalue (`|SpawnActorFromClass` "/Game/EquipoArte/Blueprints/BP_SombraAliEquipoArte.BP_SombraAliEquipoArte_C" (`|GetArrayItem` (`self.PositionData`)) "Undefined" "MultiplyWithRoot" null null))
  (set `self.AfterImageRef` _returnvalue)
  ; Pendiente: estela tras el personaje
  (`NiagaraFunctionLibrary.SpawnSystemAttached` "/Game/Lluis/VFX/NS_TrailEffect.NS_TrailEffect" (`Actor.RootComponent` (`self.GetOwner`)) "None" (-50.0 0.0 -80.0) (struct) "KeepRelativeOffset"))

(event `self.ReceiveTick`
  (params (DeltaSeconds :type "Float (single-precision)"))
  (bind _output_location (`KismetMathLibrary.BreakTransform` (`|GetArrayItem` (`self.PositionData`))))
  (`PawnMovementComponent.AddInputVector` (`Character.CharacterMovement` (`self.AfterImageRef`)) (- _output_location (`Actor.K2_GetActorLocation` (`self.AfterImageRef`))) false))

(event `Key|C`
  (params (Key :type "Key Structure"))
  (:`Pressed`
    (set `self.PlayerPos` (`Actor.K2_GetActorLocation` (`self.GetOwner`)))
    (set `self.ShadowPos` (`Actor.K2_GetActorLocation` (`self.AfterImageRef`)))
    (`Actor.K2_SetActorLocation` (`self.AfterImageRef`) (`self.PlayerPos`) false false)
    (`Actor.K2_SetActorLocation` (`GameplayStatics.GetPlayerCharacter` 0) (`self.ShadowPos`) false false)))

(fn `InitializePositionData`
  (locals (ArraySize :type Integer))
  (bind _output_get (set `local.ArraySize` (`KismetMathLibrary.Round` (/ (`self.TiempoRetraso`) 0.1))))
  (for _index (range _output_get)
    (`KismetArrayLibrary.Array_Insert` (`self.PositionData`) (`Actor.GetTransform` (`self.GetOwner`)) _index))
  (`KismetArrayLibrary.Array_Resize` (`self.PositionData`) (`local.ArraySize`)))

(fn `UpdatePositionData`
  (`KismetArrayLibrary.Array_Remove` (`self.PositionData`))
  (`KismetArrayLibrary.Array_Add` (`self.PositionData`) (`Actor.GetTransform` (`self.GetOwner`))))