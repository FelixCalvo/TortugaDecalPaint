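; BP_LuzEquipoArte is a blinking spotlight that notifies light-sensitive actors when they are lit or unlit.
; A five-second timer, set on BeginPlay and again after each toggle, flips the spotlight's visibility and its sphere's collision together.
; The sphere stands in for the lit area: begin and end overlaps send lit and unlit messages to actors implementing BPI_LightSensitive.
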(event `self.ReceiveBeginPlay`
  (bind _returnvalue (`KismetSystemLibrary.K2_SetTimerDelegate` (delegate `ToggleLight`) 5.0 true :!label _label))
  (set `self.Timer` _returnvalue))

(event `ToggleLight`
  (if (`self.IsLightOn`)
    (`SceneComponent.SetVisibility` (`self.SpotLight`) false false)
    (`PrimitiveComponent.SetCollisionEnabled` (`self.SphereCollision`) "NoCollision")
    (set `self.IsLightOn` false)
    (goto _label)
    (else
      (`SceneComponent.SetVisibility` (`self.SpotLight`) true false)
      (`PrimitiveComponent.SetCollisionEnabled` (`self.SphereCollision`) "QueryAndPhysics")
      (set `self.IsLightOn` true)
      (goto _label))))

(event `self.SphereCollision.OnComponentBeginOverlap`
  (params (OverlappedComponent :type "PrimitiveComponent Object Reference") (OtherActor :type "Actor Object Reference") (OtherComp :type "PrimitiveComponent Object Reference") (OtherBodyIndex :type Integer) (bFromSweep :type Boolean) (SweepResult :type "HitResult Structure (by ref)"))
  (if (`KismetSystemLibrary.DoesImplementInterface` OtherActor "/Game/Lluis/BluepriintInterfaces/BPI_LightSensitive.BPI_LightSensitive_C")
    (`KismetSystemLibrary.PrintString` "Illuminating something" :!enabledstate Disabled)
    (message `/Game/Lluis/BluepriintInterfaces/BPI_LightSensitive.I_SetLit` OtherActor)))

(event `self.SphereCollision.OnComponentEndOverlap`
  (params (OverlappedComponent :type "PrimitiveComponent Object Reference") (OtherActor :type "Actor Object Reference") (OtherComp :type "PrimitiveComponent Object Reference") (OtherBodyIndex :type Integer))
  (if (`KismetSystemLibrary.DoesImplementInterface` OtherActor "/Game/Lluis/BluepriintInterfaces/BPI_LightSensitive.BPI_LightSensitive_C")
    (`KismetSystemLibrary.PrintString` "no longer Illuminating something" :!enabledstate Disabled)
    (message `/Game/Lluis/BluepriintInterfaces/BPI_LightSensitive.I_SetUnlit` OtherActor)))

(fn `UserConstructionScript`)