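; Shadow actor (SombraAli) that sends itself and the player back to a checkpoint when it is hit by light.
; The checkpoint starts at the shadow's BeginPlay location and is updated through SetRespawnLocation.
; On ISetLit it moves both actors to that location and resets the trail on the player's PositionTrackerEquipoArte component.
; Both lit and unlit events print debug messages; unlit does nothing else.
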(event `/Game/Lluis/BluepriintInterfaces/BPI_LightSensitive.I_SetLit`
  (bind _returnvalue (`GameplayStatics.GetPlayerCharacter` 0))
  (bind _checkpointlocation (`self.CheckpointLocation`))
  (`KismetSystemLibrary.PrintString` "Shadow is on a light spot!!" true true (struct :`R` 1.0 :`B` 0.037799 :`A` 1.0))
  (`self.K2_SetActorLocation` _checkpointlocation)
  (`self.K2_SetActorLocation` _returnvalue _checkpointlocation false false)
  (`/Game/EquipoArte/Blueprints/PositionTrackerEquipoArte.ResetTrail` (`self.GetComponentByClass` _returnvalue "/Game/EquipoArte/Blueprints/PositionTrackerEquipoArte.PositionTrackerEquipoArte_C")))

(event `/Game/Lluis/BluepriintInterfaces/BPI_LightSensitive.I_SetUnlit`
  (`KismetSystemLibrary.PrintString` "Shadow is out of light" true true (struct :`R` 0.034841 :`G` 0.297234 :`B` 1.0 :`A` 1.0)))

(event `self.ReceiveBeginPlay`
  (set `self.CheckpointLocation` (`self.K2_GetActorLocation`)))

(event `/Game/Lluis/BluepriintInterfaces/BPI_Respawnable.SetRespawnLocation`
  (params (location :type "Vector Structure"))
  (set `self.CheckpointLocation` location))

(fn `UserConstructionScript`)