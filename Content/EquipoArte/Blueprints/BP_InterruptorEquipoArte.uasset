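; BP_InterruptorEquipoArte is a switch that holds a tagged door open while the player character or its shadow (Sombra) stands on it.
; Every Tick it polls the Box for overlapping third-person character or shadow actors, calling AbrirPuerta if either is present and CerrarPuerta if neither is.
; Both events look up BP_PuertaEquipoArte by the Nombre tag and forward the call to the first match, repeating every frame.
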(event `self.ReceiveTick`
  (params (DeltaSeconds :type "Float (single-precision)"))
  (bind _returnvalue (> (`KismetArrayLibrary.Array_Length` (`PrimitiveComponent.GetOverlappingActors` (`self.Box`) "/Game/EquipoArte/Blueprints/BP_SombraAliEquipoArte.BP_SombraAliEquipoArte_C")) 0))
  (bind _returnvalue_2 (> (`KismetArrayLibrary.Array_Length` (`PrimitiveComponent.GetOverlappingActors` (`self.Box`) "/Game/EquipoArte/Blueprints/BP_ThirdPersonCharacterAliEquipoArte.BP_ThirdPersonCharacterAliEquipoArte_C")) 0))
  (`|ExecutionSequence`
    (:`then_0`
      (if _returnvalue_2
        (`KismetSystemLibrary.PrintString` "Overlap Third Person" false true (struct :`G` 1.0 :`B` 0.052975 :`A` 1.0))
        (`self.AbrirPuerta`)))
    (:`then_1`
      (if _returnvalue
        (`KismetSystemLibrary.PrintString` "Overlap Sombra" false true (struct :`R` 0.144441 :`B` 1.0 :`A` 1.0))
        (`self.AbrirPuerta`)))
    (:`then_2`
      (if (and (not _returnvalue_2) (not _returnvalue))
        (`KismetSystemLibrary.PrintString` "Cerrar puerta" false true (struct :`R` 1.0 :`B` 0.06219 :`A` 1.0))
        (`self.CerrarPuerta`)))))

(event `AbrirPuerta`
  (bind _outactors (`GameplayStatics.GetAllActorsOfClassWithTag` "/Game/EquipoArte/Blueprints/BP_PuertaEquipoArte.BP_PuertaEquipoArte_C" (`self.Nombre`)))
  (`/Game/EquipoArte/Blueprints/BP_PuertaEquipoArte.AbrirPuerta` (`|GetArrayItem` _outactors)))

(event `CerrarPuerta`
  (bind _outactors (`GameplayStatics.GetAllActorsOfClassWithTag` "/Game/EquipoArte/Blueprints/BP_PuertaEquipoArte.BP_PuertaEquipoArte_C" (`self.Nombre`)))
  (`/Game/EquipoArte/Blueprints/BP_PuertaEquipoArte.CerrarPuerta` (`|GetArrayItem` _outactors)))

(fn `UserConstructionScript`)