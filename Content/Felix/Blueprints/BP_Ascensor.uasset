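; Elevator actor that raises its Cylinder when player character 0 enters SphereCollision and lowers it after they leave.
; Overlap plays a Timeline that lerps world Z from a hard-coded base to FMovElevator, keeping X and Y.
; End overlap waits, then reverses a second Timeline to descend.
; PositionElevatorUPDOWN flips only when each move finishes, so leaving mid-rise triggers no descent.
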(event `self.SphereCollision.OnComponentBeginOverlap`
  (params (OverlappedComponent :type "PrimitiveComponent Object Reference") (OtherActor :type "Actor Object Reference") (OtherComp :type "PrimitiveComponent Object Reference") (OtherBodyIndex :type Integer) (bFromSweep :type Boolean) (SweepResult :type "HitResult Structure (by ref)"))
  ;[0 0.15 0.02743 0.5] Comment
  (if (== OtherActor (`GameplayStatics.GetPlayerCharacter` 0))
    (if (== (`self.PositionElevatorUPDOWN`) false)
      (bind (_direction _newtrack_0) (`Timeline|Timeline` :!via `PlayFromStart`)
        (:`Update`
          (bind (_returnvalue_x _returnvalue_y _returnvalue_z) (`KismetMathLibrary.BreakVector` (`KismetMathLibrary.VLerp` (`KismetMathLibrary.MakeVector` (.x (.location (`SceneComponent.K2_GetComponentToWorld` (`self.Cylinder`)))) (.y (.location (`SceneComponent.K2_GetComponentToWorld` (`self.Cylinder`)))) -48.0) (`KismetMathLibrary.MakeVector` (.x (.location (`SceneComponent.K2_GetComponentToWorld` (`self.Cylinder`)))) (.y (.location (`SceneComponent.K2_GetComponentToWorld` (`self.Cylinder`)))) (`self.fMovElevator`)) _newtrack_0)))
          (`SceneComponent.K2_SetWorldLocation` (`self.Cylinder`) (`KismetMathLibrary.MakeVector` _returnvalue_x _returnvalue_y _returnvalue_z) false false))
        (:`Finished`
          (set `self.PositionElevatorUPDOWN` true))))))

(event `self.SphereCollision.OnComponentEndOverlap`
  (params (OverlappedComponent :type "PrimitiveComponent Object Reference") (OtherActor :type "Actor Object Reference") (OtherComp :type "PrimitiveComponent Object Reference") (OtherBodyIndex :type Integer))
  ;[0 0.15 0.02761 0.5] Bajada del ascensor
  (if (== OtherActor (`GameplayStatics.GetPlayerCharacter` 0))
    (if (== (`self.PositionElevatorUPDOWN`) true)
      (`KismetSystemLibrary.Delay` 4.1) ; Tiempo de espera hasta que empieza a bajar
      (bind (_direction _newtrack_0) (`Timeline|Timeline_0` :!via `ReverseFromEnd`) ; 5 segundos
        (:`Update`
          (bind (_returnvalue_x _returnvalue_y _returnvalue_z) (`KismetMathLibrary.BreakVector` (`KismetMathLibrary.VLerp` (`KismetMathLibrary.MakeVector` (.x (.location (`SceneComponent.K2_GetComponentToWorld` (`self.Cylinder`)))) (.y (.location (`SceneComponent.K2_GetComponentToWorld` (`self.Cylinder`)))) -48.0) (`KismetMathLibrary.MakeVector` (.x (.location (`SceneComponent.K2_GetComponentToWorld` (`self.Cylinder`)))) (.y (.location (`SceneComponent.K2_GetComponentToWorld` (`self.Cylinder`)))) (`self.fMovElevator`)) _newtrack_0)))
          (`SceneComponent.K2_SetWorldLocation` (`self.Cylinder`) (`KismetMathLibrary.MakeVector` _returnvalue_x _returnvalue_y _returnvalue_z) false false))
        (:`Finished`
          (set `self.PositionElevatorUPDOWN` false))))))

(fn `UserConstructionScript`)