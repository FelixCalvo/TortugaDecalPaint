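; Floor switch that opens a door while the player character or the shadow (Sombra) stands in its Box, and closes it when neither does.
; Tick polls overlapping actors and calls open or close every frame.
; A parallel test without Tick tracks both occupants with booleans on overlap events, firing the same calls.
; The target is the first BP_PuertaEquipoArte whose tag matches Nombre.
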(event `self.ReceiveTick`
  (params (DeltaSeconds :type "Float (single-precision)"))
  (bind _returnvalue (> (`KismetArrayLibrary.Array_Length` (`PrimitiveComponent.GetOverlappingActors` (`self.Box`) "/Game/EquipoArte/Blueprints/BP_SombraAliEquipoArte.BP_SombraAliEquipoArte_C")) 0))
  (bind _returnvalue_2 (> (`KismetArrayLibrary.Array_Length` (`PrimitiveComponent.GetOverlappingActors` (`self.Box`) "/Game/EquipoArte/Blueprints/BP_ThirdPersonCharacterAliEquipoArte.BP_ThirdPersonCharacterAliEquipoArte_C")) 0))
  (`|ExecutionSequence`
    (:`then_0`
      (if _returnvalue_2
        (`KismetSystemLibrary.PrintString` "Overlap Third Person" false true (struct :`G` 1.0 :`B` 0.052975 :`A` 1.0))
        (`self.AbrirPuerta`)))
    (:`then_1`
      (if _returnvalue
        (`KismetSystemLibrary.PrintString` "Overlap Sombra" false true (struct :`R` 0.144441 :`B` 1.0 :`A` 1.0))
        (`self.AbrirPuerta`)))
    (:`then_2`
      (if (and (not _returnvalue_2) (not _returnvalue))
        (`KismetSystemLibrary.PrintString` "Cerrar puerta" false true (struct :`R` 1.0 :`B` 0.06219 :`A` 1.0))
        (`self.CerrarPuerta`)))))

(event `AbrirPuerta`
  (bind _outactors (`GameplayStatics.GetAllActorsOfClassWithTag` "/Game/EquipoArte/Blueprints/BP_PuertaEquipoArte.BP_PuertaEquipoArte_C" (`self.Nombre`)))
  (`/Game/EquipoArte/Blueprints/BP_PuertaEquipoArte.AbrirPuerta` (`|GetArrayItem` _outactors)))

(event `CerrarPuerta`
  (bind _outactors (`GameplayStatics.GetAllActorsOfClassWithTag` "/Game/EquipoArte/Blueprints/BP_PuertaEquipoArte.BP_PuertaEquipoArte_C" (`self.Nombre`)))
  (`/Game/EquipoArte/Blueprints/BP_PuertaEquipoArte.CerrarPuerta` (`|GetArrayItem` _outactors)))

(event `self.Box.OnComponentBeginOverlap`
  (params (OverlappedComponent :type "PrimitiveComponent Object Reference") (OtherActor :type "Actor Object Reference") (OtherComp :type "PrimitiveComponent Object Reference") (OtherBodyIndex :type Integer) (bFromSweep :type Boolean) (SweepResult :type "HitResult Structure (by ref)"))
  (bind _returnvalue (`GameplayStatics.GetObjectClass` OtherActor))
  ;[0 0.15 0.02738 0.5] Prueba sin usar tick
  (if (== _returnvalue "/Game/EquipoArte/Blueprints/BP_ThirdPersonCharacterAliEquipoArte.BP_ThirdPersonCharacterAliEquipoArte_C")
    (`KismetSystemLibrary.PrintString` "Hello soy el player")
    (bind _output_get (set `self.PisandoInterruptorPlayer` true))
    (if (or (== _output_get true) (== (stale _output_get_2) true)) :!label _label
      (`self.AbrirPuerta`))
    (elif (== _returnvalue "/Game/EquipoArte/Blueprints/BP_SombraAliEquipoArte.BP_SombraAliEquipoArte_C")
      (`KismetSystemLibrary.PrintString` "Hello, soy la sombra")
      (bind _output_get_2 (set `self.PisandoInterruptorSombra` true))
      (goto _label))))

(event `self.Box.OnComponentEndOverlap`
  (params (OverlappedComponent :type "PrimitiveComponent Object Reference") (OtherActor :type "Actor Object Reference") (OtherComp :type "PrimitiveComponent Object Reference") (OtherBodyIndex :type Integer))
  (bind _returnvalue (`GameplayStatics.GetObjectClass` OtherActor))
  ;[0 0.15 0.02738 0.5] Prueba sin usar tick
  (if (== _returnvalue "/Game/EquipoArte/Blueprints/BP_ThirdPersonCharacterAliEquipoArte.BP_ThirdPersonCharacterAliEquipoArte_C")
    (`KismetSystemLibrary.PrintString` "Bajando el player")
    (bind _output_get (set `self.PisandoInterruptorPlayer` false))
    (if (and (== false _output_get) (== (stale _output_get_2) false)) :!label _label_2
      (`self.CerrarPuerta`))
    (elif (== _returnvalue "/Game/EquipoArte/Blueprints/BP_SombraAliEquipoArte.BP_SombraAliEquipoArte_C")
      (`KismetSystemLibrary.PrintString` "Bajando la sombra")
      (bind _output_get_2 (set `self.PisandoInterruptorSombra` false))
      (goto _label_2))))

(fn `UserConstructionScript`)